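; BP_Sun is a sun actor whose surface material animates its shine.
; The construction script creates a dynamic material instance from the Sun component's first material.
; On BeginPlay, the SunShine timeline plays at half speed and feeds its scaled value into that material's Shining scalar parameter.
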(event EventBeginPlay
  (Components|Timeline|SetPlayRate (Variables|Default|GetSunShine) 0.5)
  (bind _shining (Timeline|SunShine Play)
    (:Update
      (Rendering|Material|SetScalarParameterValue (Variables|Default|GetMID_Sun) "Shining" (* _shining 7.0) :!class /Script/Engine.MaterialInstanceDynamic))))

(event Collision|EventActorBeginOverlap
  (params (OtherActor :type Actor%20Object%20Reference)))

(event EventTick
  (params (DeltaSeconds :type Float%20%28single-precision%29)))

(fn ConstructionScript
  (bind _sun (Variables|Default|GetSun))
  (bind _returnvalue (Rendering|Material|CreateDynamicMaterialInstance _sun 0 (Rendering|Material|GetMaterial _sun 0) "None" :!class /Script/Engine.PrimitiveComponent))
  (Variables|Default|SetMID_Sun _returnvalue))